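; Animation notify state that keeps a character with a combo component in the air for the span of the notify window.
; On begin it finds BP_ComboComponent on the mesh owner and switches that component's Character to Flying movement.
; On end it sets movement to Walking rather than restoring the previous mode.
; Without a valid combo component both events change nothing and return false, and tick does no work.
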(fn ReceivedNotifyBegin
  (params (MeshComp :type Skeletal%20Mesh%20Component%20Object%20Reference) (Animation :type Anim%20Sequence%20Base%20Object%20Reference) (TotalDuration :type Float%20%28single-precision%29))
  (bind _returnvalue (Components|GetOwner MeshComp))
  (bind _returnvalue_2 (Actor|GetComponentbyClass _returnvalue "/Game/ComboComponent/Blueprints/Components/BP_ComboComponent.BP_ComboComponent_C"))
  ;[1 0.8011 0.2045] Allows for the input of the next Combo Element  (Also starts the timer to detect a delay)
  (Utilities|IsValid _returnvalue_2
    (:Is%20Valid
      (Pawn|Components|CharacterMovement|SetMovementMode (Variables|/Script/Engine.Character|GetCharacterMovement (Variables|/Game/ComboComponent/Blueprints/Components/BP_ComboComponent.BP_ComboComponent_C|GetCharacter _returnvalue_2)) "MOVE_Flying" 0)
      (return true))
    (:Is%20Not%20Valid
      (return false))))

(fn ReceivedNotifyEnd
  (params (MeshComp :type Skeletal%20Mesh%20Component%20Object%20Reference) (Animation :type Anim%20Sequence%20Base%20Object%20Reference))
  (bind _returnvalue (Components|GetOwner MeshComp))
  (bind _returnvalue_2 (Actor|GetComponentbyClass _returnvalue "/Game/ComboComponent/Blueprints/Components/BP_ComboComponent.BP_ComboComponent_C"))
  ;[1 0.8011 0.2045] Checks if the Combo should continue or not. If not, fail the combo
  (Utilities|IsValid _returnvalue_2
    (:Is%20Valid
      (Pawn|Components|CharacterMovement|SetMovementMode (Variables|/Script/Engine.Character|GetCharacterMovement (Variables|/Game/ComboComponent/Blueprints/Components/BP_ComboComponent.BP_ComboComponent_C|GetCharacter _returnvalue_2)) "MOVE_Walking" 0)
      (return true))
    (:Is%20Not%20Valid
      (return false))))

(fn ReceivedNotifyTick
  (params (MeshComp :type Skeletal%20Mesh%20Component%20Object%20Reference) (Animation :type Anim%20Sequence%20Base%20Object%20Reference) (FrameDeltaTime :type Float%20%28single-precision%29))
  (return false))