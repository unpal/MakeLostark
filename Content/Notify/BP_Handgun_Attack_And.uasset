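; Animation notify that marks a point in the handgun general attack, apparently its end ("And"), on a TopDownCharacter.
; It casts the mesh owner and its controller, then checks two attack counters on the character's HandgunL.
; It re-enables the player controller's Move flag unless those counters fall in a range that suggests a combo still running.
; In either case it then calls GeneralAttackAnd on HandgunL.
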(fn ReceivedNotify
  (params (MeshComp :type Skeletal%20Mesh%20Component%20Object%20Reference) (Animation :type Anim%20Sequence%20Base%20Object%20Reference))
  (bind _astop_down_character (Utilities|Casting|CastToTopDownCharacter (Components|GetOwner MeshComp)))
  (bind _astest_player_controller (Utilities|Casting|CastTotestPlayerController (Pawn|GetController _astop_down_character)))
  (if (and (< (Variables|/Script/test.Handgun_Stance|GetGeneral_Attack_And_Count (Variables|/Script/test.testCharacter|GetHandgun_L _astop_down_character)) 3) (> (Variables|/Script/test.Handgun_Stance|GetGeneral_Attack_Count (Variables|/Script/test.testCharacter|GetHandgun_L _astop_down_character)) 1))
    _
    (else
      (Variables|/Script/test.testPlayerController|SetbMove _astest_player_controller true)))
  (Class|HandgunStance|GeneralAttackand (Variables|/Script/test.testCharacter|GetHandgun_L _astop_down_character))
  (return false))