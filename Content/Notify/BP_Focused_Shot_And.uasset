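; BP_Focused_Shot_And is an anim notify that chains the follow-up montage in the Focused Shot combo for the TopDownCharacter.
; On trigger it reads FocusedShotComboCount from the owner's testPlayerController.
; While the count is below one it plays the Gunslinger Attack03 montage and increments the count, otherwise it plays the Combo04_2 montage.
; The notify never resets the counter.
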(fn ReceivedNotify
  (params (MeshComp :type Skeletal%20Mesh%20Component%20Object%20Reference) (Animation :type Anim%20Sequence%20Base%20Object%20Reference))
  (bind _astop_down_character (Utilities|Casting|CastToTopDownCharacter (Components|GetOwner MeshComp)))
  (bind _astest_player_controller (Utilities|Casting|CastTotestPlayerController (Pawn|GetController _astop_down_character)))
  (if (< (Variables|/Script/test.testPlayerController|GetFocused_Shot_Combo_Count _astest_player_controller) 1)
    (Animation|PlayAnimMontage _astop_down_character "/Game/Montage/Frank_RPG_Gunslinger_Attack03_Montage.Frank_RPG_Gunslinger_Attack03_Montage" 1.0 "None")
    (Variables|/Script/test.testPlayerController|SetFocused_Shot_Combo_Count _astest_player_controller (+ (Variables|/Script/test.testPlayerController|GetFocused_Shot_Combo_Count _astest_player_controller) 1))
    (else
      (Animation|PlayAnimMontage _astop_down_character "/Game/Montage/Frank_RPG_Gunslinger_Combo04_2_Montage.Frank_RPG_Gunslinger_Combo04_2_Montage" 1.0 "None")))
  (return false))