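; Animation notify that chains the PeaceKeeper combo attack montages on the TopDownCharacter.
; When fired, it reads input and combo counters on the owner's testPlayerController.
; If more than two inputs are buffered and the combo is below its cap, it clears inputs, advances the combo and plays the second or third montage.
; With too few inputs, it resets both counters and clears the IsESkill flag.
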(fn ReceivedNotify
  (params (MeshComp :type Skeletal%20Mesh%20Component%20Object%20Reference) (Animation :type Anim%20Sequence%20Base%20Object%20Reference))
  (bind _astop_down_character (Utilities|Casting|CastToTopDownCharacter (Components|GetOwner MeshComp)))
  (bind _astest_player_controller (Utilities|Casting|CastTotestPlayerController (Pawn|GetController _astop_down_character)))
  (if (> (Variables|/Script/test.testPlayerController|GetPeaceKeeper_Input_Count _astest_player_controller) 2)
    (if (< (Variables|/Script/test.testPlayerController|GetPeaceKeeper_Combo_Count _astest_player_controller) 2)
      (Variables|/Script/test.testPlayerController|SetPeaceKeeper_Input_Count _astest_player_controller 0)
      (Variables|/Script/test.testPlayerController|SetPeaceKeeper_Combo_Count _astest_player_controller (+ (Variables|/Script/test.testPlayerController|GetPeaceKeeper_Combo_Count _astest_player_controller) 1))
      (if (== (Variables|/Script/test.testPlayerController|GetPeaceKeeper_Combo_Count _astest_player_controller) 1)
        (Animation|PlayAnimMontage _astop_down_character "/Game/Montage/PeaceKeeper_Anim_Montage_2.PeaceKeeper_Anim_Montage_2" 2.0 "None")
        (elif (== (Variables|/Script/test.testPlayerController|GetPeaceKeeper_Combo_Count _astest_player_controller) 2)
          (Animation|PlayAnimMontage _astop_down_character "/Game/Montage/Peacekeeper_Anim_Montage_3.Peacekeeper_Anim_Montage_3" 1.3 "None")
          (else
            (Animation|PlayAnimMontage _astop_down_character "/Game/Montage/Peacekeeper_Anim_Montage_3.Peacekeeper_Anim_Montage_3" 2.0 "None"))))
      (return false))
    (else
      (Variables|/Script/test.testPlayerController|SetPeaceKeeper_Input_Count _astest_player_controller 0)
      (Variables|/Script/test.testPlayerController|SetPeaceKeeper_Combo_Count _astest_player_controller 0)
      (Variables|/Script/test.testPlayerController|SetIs_E_Skill _astest_player_controller false)
      (return false))))