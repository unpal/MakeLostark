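; BP_Dash_End is an animation notify that sets the current weapon's GeneralAttack flag when a dash animation reaches it.
; It casts the mesh owner to TopDownCharacter and its controller to testPlayerController, acting only while DashCount is below one.
; It branches on handgun, shotgun or rifle stance, also resetting the left handgun's attack counters or the controller's focused-shot state and combo count for rifle.
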(fn ReceivedNotify
  (params (MeshComp :type Skeletal%20Mesh%20Component%20Object%20Reference) (Animation :type Anim%20Sequence%20Base%20Object%20Reference))
  (bind _astop_down_character (Utilities|Casting|CastToTopDownCharacter (Components|GetOwner MeshComp)))
  (bind _astest_player_controller (Utilities|Casting|CastTotestPlayerController (Pawn|GetController _astop_down_character)))
  (if (< (Variables|/Script/test.testPlayerController|GetDashCount _astest_player_controller) 1)
    (if (Variables|/Script/test.testCharacter|GetHandgunStance _astop_down_character)
      (Variables|/Script/test.Handgun_Stance|SetbGeneral_Attack (Variables|/Script/test.testCharacter|GetHandgun_L _astop_down_character) true)
      (Variables|/Script/test.Handgun_Stance|SetGeneral_Attack_And_Count (Variables|/Script/test.testCharacter|GetHandgun_L _astop_down_character) 0)
      (Variables|/Script/test.Handgun_Stance|SetGeneral_Attack_Count (Variables|/Script/test.testCharacter|GetHandgun_L _astop_down_character) 0)
      (return false)
      (elif (Variables|/Script/test.testCharacter|GetShotgunStance _astop_down_character)
        (Variables|/Script/test.Shotgun_Stance|SetbGeneral_Attack (Variables|/Script/test.testCharacter|GetShotgun _astop_down_character) true)
        (return false)
        (elif (Variables|/Script/test.testCharacter|GetRifleStance _astop_down_character)
          (Variables|/Script/test.Rifle_Stance|SetbGeneral_Attack (Variables|/Script/test.testCharacter|GetRifle _astop_down_character) true)
          (Variables|/Script/test.testPlayerController|SetIsFocused_Shot _astest_player_controller false)
          (Variables|/Script/test.testPlayerController|SetFocused_Shot_Combo_Count _astest_player_controller 0)
          (return false))))))