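; BP_ComboNotifyState is an animation notify state that marks the window in a montage or animation where the owner's next combo input is accepted.
; On begin, unless the element is a finisher, it sets CanCombo on the owner's BP_ComboComponent, starts the delay timer and tries the next AI combo.
; On end, if CanCombo remains set and no delayed follow-up is pending, it resets finishers or fails the combo.
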(fn ReceivedNotifyBegin
  (params (MeshComp :type Skeletal%20Mesh%20Component%20Object%20Reference) (Animation :type Anim%20Sequence%20Base%20Object%20Reference) (TotalDuration :type Float%20%28single-precision%29))
  (bind _returnvalue (Components|GetOwner MeshComp))
  (bind _returnvalue_2 (Actor|GetComponentbyClass _returnvalue "/Game/ComboComponent/Blueprints/Components/BP_ComboComponent.BP_ComboComponent_C"))
  ;[1 0.8011 0.2045] Allows for the input of the next Combo Element  (Also starts the timer to detect a delay)
  (Utilities|IsValid _returnvalue_2
    (:Is%20Valid
      (if (Default|IsElemFinisher? _returnvalue_2)
        _
        (else
          (Variables|/Game/ComboComponent/Blueprints/Components/BP_ComboComponent.BP_ComboComponent_C|SetCanCombo? _returnvalue_2 true)
          (Default|StartComboTimer _returnvalue_2)
          (Default|TryNextAICombo _returnvalue_2)
          (return true))))
    (:Is%20Not%20Valid
      _))
  (return false))

(fn ReceivedNotifyEnd
  (params (MeshComp :type Skeletal%20Mesh%20Component%20Object%20Reference) (Animation :type Anim%20Sequence%20Base%20Object%20Reference))
  (bind _returnvalue (Components|GetOwner MeshComp))
  (bind _returnvalue_2 (Actor|GetComponentbyClass _returnvalue "/Game/ComboComponent/Blueprints/Components/BP_ComboComponent.BP_ComboComponent_C"))
  ;[1 0.8011 0.2045] Checks if the Combo should continue or not. If not, fail the combo
  (Utilities|IsValid _returnvalue_2
    (:Is%20Valid
      (if (Variables|/Game/ComboComponent/Blueprints/Components/BP_ComboComponent.BP_ComboComponent_C|GetCanCombo? _returnvalue_2)
        (if (and (Default|PotentialHasDelay? _returnvalue_2 (Variables|/Game/ComboComponent/Blueprints/Components/BP_ComboComponent.BP_ComboComponent_C|GetCurrentComboIndex _returnvalue_2)) (Variables|/Game/ComboComponent/Blueprints/Components/BP_ComboComponent.BP_ComboComponent_C|GetTimerActive? _returnvalue_2))
          _
          (else
            (if (Default|IsElemFinisher? _returnvalue_2)
              (Default|ResetCombo _returnvalue_2)
              (else
                (Default|FailCombo _returnvalue_2)))
            (return true))))
      (return true))
    (:Is%20Not%20Valid
      (return false))))